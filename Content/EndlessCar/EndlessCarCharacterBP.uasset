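; Player character for an endless car game that drives forward automatically and strafes sideways on input.
; Tick adds constant movement input along the control rotation's yaw.
; The MoveRight axis plays one of two timelines that lerp the actor location from a cached start to a fixed side and forward offset, without sweep.
; CanGoRight and CanGoLeft flags block repeating the same direction until its timeline finishes, while allowing the opposite one.
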(event `self.ReceiveBeginPlay`
  (set `self.CanGoRight?` true))

(event `self.ReceiveTick`
  (params (DeltaSeconds :type "Float (single-precision)"))
  (`self.AddMovementInput` (`KismetMathLibrary.GetForwardVector` (`KismetMathLibrary.MakeRotator` 0.0 0.0 (.yaw (`self.GetControlRotation`))))))

(event `InputAxis|MoveRight`
  (params (AxisValue :type "Float (single-precision)"))
  (if (and (`self.CanGoRight?`) (> AxisValue 0.0))
    (bind _output_get (set `self.CarLocation` (`self.K2_GetActorLocation`)))
    (set `self.CanGoRight?` false)
    (set `self.CanGoLeft?` true)
    (bind (_direction _alpha) (`Timeline|StrafeRIghtTimeline` :!via `PlayFromStart`)
      (:`Update`
        (`self.K2_SetActorLocation` (`KismetMathLibrary.VLerp` _output_get (`KismetMathLibrary.MakeVector` (+ (.x _output_get) 150.0) (+ (.y _output_get) 350.0) (.z _output_get)) _alpha)))
      (:`Finished`
        (set `self.CanGoRight?` true)))
    (elif (and (`self.CanGoLeft?`) (< AxisValue 0.0))
      (bind _output_get_2 (set `self.CarLocation` (`self.K2_GetActorLocation`)))
      (set `self.CanGoRight?` true)
      (set `self.CanGoLeft?` false)
      (bind (_direction_2 _alpha_2) (`Timeline|Timeline_0` :!via `PlayFromStart`)
        (:`Update`
          (`self.K2_SetActorLocation` (`KismetMathLibrary.VLerp` _output_get_2 (`KismetMathLibrary.MakeVector` (+ (.x _output_get_2) 150.0) (+ (.y _output_get_2) -350.0) (.z _output_get_2)) _alpha_2)))
        (:`Finished`
          (set `self.CanGoLeft?` true))))))

(fn `UserConstructionScript`)