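; AI-driven car character for the EndlessCar game that drives straight ahead and kills the player car on contact.
; Each Tick it sets movement velocity along the capsule's forward vector at a fixed km/h speed converted to cm/s, and also adds forward movement input.
; A static mesh hit on an EndlessCarCharacterBP calls that character's DeathEvent.
; It contains no steering or avoidance logic.
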(event `self.ReceiveBeginPlay`)

(event `self.ReceiveTick`
  (params (DeltaSeconds :type "Float (single-precision)"))
  (bind _returnvalue (`SceneComponent.GetForwardVector` (`self.CapsuleComponent`)))
  (set `MovementComponent.Velocity` (* _returnvalue (* 30.0 (/ 1000.0 36.0))) (`self.CharacterMovement`))
  (`self.AddMovementInput` _returnvalue))

(event `self.StaticMesh.OnComponentHit`
  (params (HitComponent :type "PrimitiveComponent Object Reference") (OtherActor :type "Actor Object Reference") (OtherComp :type "PrimitiveComponent Object Reference") (NormalImpulse :type "Vector Structure") (Hit :type "HitResult Structure (by ref)"))
  (bind _asendless_car_character_bp (cast `/Game/EndlessCar/EndlessCarCharacterBP` OtherActor))
  (`/Game/EndlessCar/EndlessCarCharacterBP.DeathEvent` _asendless_car_character_bp))

(fn `UserConstructionScript`)